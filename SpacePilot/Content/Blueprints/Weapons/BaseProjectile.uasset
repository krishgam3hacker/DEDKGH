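; Base projectile Blueprint for weapons that flies straight forward and damages any BaseShip it hits.
; Each Tick it line traces the next step on the Camera channel, ignoring its instigator, then moves by Speed without sweep or delta-time scaling.
; A BaseShip hit receives Damage and prints a debug message, and the projectile is not destroyed.
; Trace debug drawing is left on.
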(event EventBeginPlay)

(event Collision|EventActorBeginOverlap
  (params (OtherActor :type Actor%20Object%20Reference)))

(event EventTick
  (params (DeltaSeconds :type Float%20%28single-precision%29))
  (bind _returnvalue (Transformation|GetActorLocation))
  (bind _returnvalue_2 (Transformation|GetActorForwardVector))
  (bind _speed (Variables|Default|GetSpeed))
  (bind _returnvalue_3 (* _returnvalue_2 _speed))
  (bind _returnvalue_4 (+ _returnvalue _returnvalue_3))
  (bind _outhit (Collision|LineTraceByChannel _returnvalue _returnvalue_4 "TraceTypeQuery2" false (Utilities|Array|MakeArray (Game|GetInstigator)) "ForDuration"))
  (Transformation|SetActorLocation _returnvalue_4 false false)
  (bind _asbase_ship (Utilities|Casting|CastToBaseShip (.HitActor (Collision|BreakHitResult _outhit))))
  (Game|Damage|ApplyDamage _asbase_ship (Variables|Default|GetDamage) 0 0)
  (Development|PrintString "Hit enemy"))

(fn ConstructionScript)