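; AI ship enemy that wanders between seven Arrow components while its Cube spins in yaw every tick.
; FindNextLocation picks a random arrow's world location and a new random spin rate, starts Moving, then repeats after a short random delay.
; Moving re-arms its own timer and lerps the Cube from its current location by a fixed fraction each step, producing an eased approach to the target.
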(event Custom|Moving
  (bind _cube (Variables|Default|GetCube))
  (Variables|Default|SetAlpha 0.0)
  (Utilities|Time|SetTimerbyEvent (delegate Custom|Moving) 0.02)
  (Variables|Default|SetAlpha (+ (Variables|Default|GetAlpha) 0.04))
  (Transformation|SetWorldLocation _cube (Math|Vector|Lerp(Vector) (Transformation|GetWorldLocation _cube) (Variables|Default|GetLocation%20to%20Move) (Variables|Default|GetAlpha)) false false))

(event Custom|FindNextLocation
  (bind _arrow (Variables|Default|GetArrow))
  (bind _arrow1 (Variables|Default|GetArrow1))
  (bind _arrow2 (Variables|Default|GetArrow2))
  (bind _arrow3 (Variables|Default|GetArrow3))
  (bind _arrow4 (Variables|Default|GetArrow4))
  (bind _arrow5 (Variables|Default|GetArrow5))
  (bind _arrow6 (Variables|Default|GetArrow6))
  (bind _array (Utilities|Array|MakeArray _arrow _arrow1 _arrow2 _arrow3 _arrow4 _arrow5 _arrow6))
  (Variables|Default|SetDelta%20Rotation%20Z%20%28Yaw%29 (Math|Random|RandomFloatinRange -5.0 5.0))
  (Variables|Default|SetLocation%20to%20Move (Transformation|GetWorldLocation (Utilities|Array|Get(acopy) _array (Math|Random|RandomIntegerinRange 0 (Utilities|Array|LastIndex _array)))))
  (CallFunction|Moving)
  (Utilities|FlowControl|Delay (Math|Random|RandomFloatinRange 1.5 2.5))
  (CallFunction|FindNextLocation))

(event EventBeginPlay
  (CallFunction|FindNextLocation))

(event Collision|EventActorBeginOverlap
  (params (OtherActor :type Actor%20Object%20Reference)))

(event EventTick
  (params (DeltaSeconds :type Float%20%28single-precision%29))
  (Transformation|AddLocalRotation (Variables|Default|GetCube) (Math|Rotator|MakeRotator 0.0 0.0 (Variables|Default|GetDelta%20Rotation%20Z%20%28Yaw%29)) false false))

(fn ConstructionScript)